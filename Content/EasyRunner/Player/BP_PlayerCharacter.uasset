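; Player character for an endless runner that constantly moves forward along its control rotation and gains a coin about every second.
; Setup events walk it to a start location, snap its position and rotation, enable Tick after a delay, and blend to its camera.
; Damage reduces health; death fires a dispatcher, shows the HUD game-over screen and requests a save.
; The game instance handles coin persistence, and pause input forwards to the HUD.
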(event `OnTestDelegate_Event`
  (`KismetSystemLibrary.PrintString` "Hello"))

(event `self.ReceiveBeginPlay`
  (`|ExecutionSequence`
    (:`then_0`
      ;[1 1 1] Lowest should be -0.5 (-0.375 means half regular speed: 0.75 - 0.375 = 0.375)
      (set `self.maxDeceleration` -0.375)
      (add `self.OnTestDelegate` (delegate `OnTestDelegate_Event`)))
    (:`then_1`
      ;[1 1 1] Max effect is 0.25
      (set `self.maxAceleration` 0.25))
    (:`then_2`
      ;[1 1 1] This is effectively our 'game speed'... increase it as time goes on
      (set `CharacterMovementComponent.MaxWalkSpeed` 500.0 (`self.CharacterMovement`)))
    (:`then_3`
      ;[1 1 1] Setting initial health
      (set `self.Health` (`self.MaxHealth`)))
    (:`then_4`
      (message `/Game/EasyRunner/SaveGameSystem/BPI_Persistence.RequestLoadGivenObject` (`GameplayStatics.GetGameInstance`) self))))

(event `self.ReceiveTick`
  (params (DeltaSeconds :type "Float (single-precision)"))
  ;[1 1 1] Infinitly running forwards
  (`self.AddMovementInput` (`KismetMathLibrary.GetForwardVector` (`self.GetControlRotation`)) 0.75)
  (`KismetSystemLibrary.Delay` 1.0)
  (bind _result (`/Engine/EditorBlueprintResources/StandardMacros.IncrementInt` (`self.Coins`))
    (:`  `
      (`KismetSystemLibrary.PrintString` (`KismetStringLibrary.Conv_IntToString` _result)))))

(event `self.ReceiveAnyDamage`
  (params (Damage :type "Float (single-precision)") (DamageType :type "DamageType Object Reference") (InstigatedBy :type "Controller Object Reference") (DamageCauser :type "Actor Object Reference"))
  ;[1 1 1] Basic Damage System
  (bind _output_get (set `self.Health` (- (`self.Health`) Damage)))
  (if (< _output_get 0.001)
    (`self.OnPlayerDeath`)
    (message `/Game/EasyRunner/UI/BPI_UIManagerCommunication.DisplayGameOverScreen` (`PlayerController.GetHUD` (`GameplayStatics.GetPlayerController` 0)))
    (message `/Game/EasyRunner/SaveGameSystem/BPI_Persistence.RequestSaveGame` (`GameplayStatics.GetGameInstance`) true)))

(event `EnhancedInput|/Game/EasyRunner/Input/Actions/IA_PauseGame`
  (params (ActionValue :type Boolean) (ElapsedSeconds :type "Float (double-precision)") (TriggeredSeconds :type "Float (double-precision)") (InputAction :type "InputAction Object Reference" :default "/Game/EasyRunner/Input/Actions/IA_PauseGame.IA_PauseGame"))
  ;[1 1 1] Pauses the game by calling the pause game function on our hud class
  (:`Started`
    (message `/Game/EasyRunner/UI/BPI_UIManagerCommunication.PauseTheGame` (`PlayerController.GetHUD` (`GameplayStatics.GetPlayerController` 0)))))

(event `/Game/EasyRunner/Player/BPI_WorldToPlayerCommunication.MoveToStartingLocation`
  (params (StartingLocation :type "Vector Structure"))
  ;[1 1 1] Moves the actor to a given location (rough precision)
  (`AIBlueprintHelperLibrary.SimpleMoveToLocation` (`self.GetController`) StartingLocation))

(event `/Game/EasyRunner/Player/BPI_WorldToPlayerCommunication.SetInitialPositionAndRunningDirection`
  (params (InitialStartingPos :type "Transform Structure"))
  (bind _returnvalue (`self.GetController`))
  (bind _rotation (.rotation InitialStartingPos))
  (bind (_returnvalue_x _returnvalue_y _returnvalue_z) (`KismetMathLibrary.BreakVector` (`self.K2_GetActorLocation`)))
  ;[1 1 1] Stop all movement then setup the players initial rotation, position and control rotation
  (`Controller.StopMovement` _returnvalue)
  (`Controller.SetControlRotation` _returnvalue _rotation)
  (`self.K2_SetActorLocationAndRotation` (+ (.location InitialStartingPos) (`KismetMathLibrary.MakeVector` 0.0 0.0 _returnvalue_z)) _rotation true)
  (`KismetSystemLibrary.Delay` 3.0)
  (`self.SetActorTickEnabled` true))

(event `/Game/EasyRunner/Player/BPI_WorldToPlayerCommunication.ActivatePlayerCamera`
  ;[1 1 1] Set this actors camera as the view target
  (`PlayerController.SetViewTargetWithBlend` (`GameplayStatics.GetPlayerController` 0) self 3.0 "VTBlend_Cubic" 0.33 false))

(event `/Game/EasyRunner/SaveGameSystem/BPI_Savable.SaveData`
  (params (SaveGameRef :type "/Game/EasyRunner/SaveGameSystem/BP_SaveGame Object Reference"))
  ;[1 1 1] Save and Load Player Data
  (set `/Game/EasyRunner/SaveGameSystem/BP_SaveGame.Coins` (`self.Coins`) SaveGameRef))

(event `/Game/EasyRunner/SaveGameSystem/BPI_Savable.LoadData`
  (params (SaveGameRef :type "/Game/EasyRunner/SaveGameSystem/BP_SaveGame Object Reference"))
  ;[1 1 1] Save and Load Player Data
  (set `self.Coins` (`/Game/EasyRunner/SaveGameSystem/BP_SaveGame.Coins` SaveGameRef)))

(fn `MoveToLocation`
  (params (TargetLocation :type "Vector Structure"))
  (`self.AddMovementInput` (- TargetLocation (`SceneComponent.K2_GetComponentLocation` (`self.CapsuleComponent`))))
  (`KismetSystemLibrary.PrintString` "Hello"))

(fn `UserConstructionScript`)