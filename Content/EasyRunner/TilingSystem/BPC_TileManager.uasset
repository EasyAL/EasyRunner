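; BPC_TileManager is the tile manager for EasyRunner, chaining track tiles endlessly while keeping only a short trail alive.
; Init spawns a starting platform and first tile, then binds to that tile's OnSpawnNextTile event.
; Each event destroys the previous tile, spawns the next at the current tile's AttachmentPoint and binds to it.
; A flip-flop boolean alternates the spawned class between BP_TileBase and BP_TileBase_Child.
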(event `/Game/EasyRunner/TilingSystem/BPI_TileManagerCommunication.Init`
  (bind _returnvalue (`|SpawnActorFromClass` "/Game/EasyRunner/TilingSystem/BP_StartingPlatform.BP_StartingPlatform_C" (`KismetMathLibrary.MakeTransform` (0.0 0.0 0.0)) "Undefined" "MultiplyWithRoot" null null))
  (bind _returnvalue_2 (`|SpawnActorFromClass` "/Game/EasyRunner/TilingSystem/BP_TileBase_Child.BP_TileBase_Child_C" (`KismetMathLibrary.MakeTransform` (`SceneComponent.K2_GetComponentLocation` (`/Game/EasyRunner/TilingSystem/BP_StartingPlatform.AttachmentPoint` _returnvalue))) "Undefined" "MultiplyWithRoot" null null))
  (bind _output_get (set `self.CurrentTile` _returnvalue_2))
  (add `/Game/EasyRunner/TilingSystem/BP_TileBase.OnSpawnNextTile` _output_get (`|CreateDelegate` :!event `SpawnNextTile`)))

(event `SpawnNextTile`
  (`self.DeleteLastTile`)
  (bind _output_get (set `self.LastTile` (`self.CurrentTile`)))
  (bind _tileclass (`self.GetNextTileToSpawn`))
  (bind _returnvalue (`|SpawnActorFromClass` _tileclass (`KismetMathLibrary.MakeTransform` (`SceneComponent.K2_GetComponentLocation` (`/Game/EasyRunner/TilingSystem/BP_TileBase.AttachmentPoint` _output_get))) "Undefined" "MultiplyWithRoot" null null))
  (bind _output_get_2 (set `self.CurrentTile` _returnvalue))
  (add `/Game/EasyRunner/TilingSystem/BP_TileBase.OnSpawnNextTile` _output_get_2 (`|CreateDelegate` :!event `SpawnNextTile`)))

(fn `DeleteLastTile`
  ;[1 1 1] Figure out how to unbind from events in the future
  (bind _lasttile (`self.LastTile`)
    (:`then`
      (`Actor.K2_DestroyActor` _lasttile))
    (:`else`)))

(fn `FlipFlopTheBool`
  (if (`self.FlipFlopBool`)
    (set `self.FlipFlopBool` false)
    (else
      (set `self.FlipFlopBool` true))))

(fn `GetNextTileToSpawn`
  (returns (TileClass :type "/Game/EasyRunner/TilingSystem/BP_TileBase Class Reference"))
  (if (`self.FlipFlopBool`)
    (`self.FlipFlopTheBool`)
    (return "/Game/EasyRunner/TilingSystem/BP_TileBase.BP_TileBase_C")
    (else
      (`self.FlipFlopTheBool`)
      (return "/Game/EasyRunner/TilingSystem/BP_TileBase_Child.BP_TileBase_Child_C"))))