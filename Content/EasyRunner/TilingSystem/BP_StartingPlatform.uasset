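; BP_StartingPlatform is the runner's starting platform actor, which takes over the player's view when play begins.
; When an actor enters its Box, it sends that actor interface messages to set its initial position and running direction from a stored transform and to activate the player camera.
; A second trigger destroys the platform after a delay once an actor implementing BPI_WorldToPlayerCommunication overlaps it.
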(event `self.ReceiveBeginPlay`
  ;[1 1 1] Steals Player View On Begin Play
  (`PlayerController.SetViewTargetWithBlend` (`GameplayStatics.GetPlayerController` 0) self 0.0 "VTBlend_Linear" 0.0 false))

(event `self.Box.OnComponentBeginOverlap`
  (params (OverlappedComponent :type "PrimitiveComponent Object Reference") (OtherActor :type "Actor Object Reference") (OtherComp :type "PrimitiveComponent Object Reference") (OtherBodyIndex :type Integer) (bFromSweep :type Boolean) (SweepResult :type "HitResult Structure (by ref)"))
  (message `/Game/EasyRunner/Player/BPI_WorldToPlayerCommunication.SetInitialPositionAndRunningDirection` OtherActor (`self.Initial Starting Transform`))
  (message `/Game/EasyRunner/Player/BPI_WorldToPlayerCommunication.ActivatePlayerCamera` OtherActor))

(event `self.DestroySelfCollisionBox.OnComponentBeginOverlap`
  (params (OverlappedComponent :type "PrimitiveComponent Object Reference") (OtherActor :type "Actor Object Reference") (OtherComp :type "PrimitiveComponent Object Reference") (OtherBodyIndex :type Integer) (bFromSweep :type Boolean) (SweepResult :type "HitResult Structure (by ref)"))
  (if (`KismetSystemLibrary.DoesImplementInterface` OtherActor "/Game/EasyRunner/Player/BPI_WorldToPlayerCommunication.BPI_WorldToPlayerCommunication_C")
    (`KismetSystemLibrary.Delay` 10.0)
    (`self.K2_DestroyActor`)))

(fn `UserConstructionScript`)